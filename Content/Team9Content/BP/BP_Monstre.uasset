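; BP_Monstre is a monster Blueprint that moves toward the corner points of a BP_Route actor, found at BeginPlay.
; Space bar triggers CE_Move, which passes the SW, SE, NE and NW world locations to CE_MoveIA back-to-back, without waiting between moves.
; CE_MoveIA runs a five-second MoveComponentTo, using each world location as a relative target.
; Print strings serve as debug output, and Tick is empty.
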(event `self.ReceiveBeginPlay`
  (bind _returnvalue (`GameplayStatics.GetActorOfClass` "/Game/Team9Content/BP/BP_Route.BP_Route_C"))
  (set `self.Route` _returnvalue))

(event `self.ReceiveTick`
  (params (DeltaSeconds :type "Float (single-precision)")))

(event `Key|SpaceBar`
  (params (Key :type "Key Structure"))
  (:`Pressed`
    (`self.CE_Move`)
    (`KismetSystemLibrary.PrintString` "space")))

(event `CE_MoveIA`
  (params (NextDirection :type "Vector Structure"))
  (`KismetSystemLibrary.MoveComponentTo` null NextDirection (struct) false false 5.0)
  (`KismetSystemLibrary.PrintString` "Hello"))

(event `CE_Move`
  (bind _route (`self.Route`))
  (`self.CE_MoveIA` (`SceneComponent.K2_GetComponentLocation` (`/Game/Team9Content/BP/BP_Route.SW` _route)))
  (`self.CE_MoveIA` (`SceneComponent.K2_GetComponentLocation` (`/Game/Team9Content/BP/BP_Route.SE` _route)))
  (`self.CE_MoveIA` (`SceneComponent.K2_GetComponentLocation` (`/Game/Team9Content/BP/BP_Route.NE` _route)))
  (`self.CE_MoveIA` (`SceneComponent.K2_GetComponentLocation` (`/Game/Team9Content/BP/BP_Route.NW` _route))))

(fn `UserConstructionScript`)