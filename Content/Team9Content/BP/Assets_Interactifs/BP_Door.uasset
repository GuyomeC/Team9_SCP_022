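; Interactive metal door actor that swings open when interacted with and closes itself after a delay.
; The Interactable event, ignored while Opened is set, starts a Timeline that lerps the door mesh's yaw through a quarter turn, with a metal sound.
; The Timeline's Update pin also feeds a Delay that replays the sound and, if still open, reverses the Timeline.
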(event `open door`
  (set `self.Opened` true)
  (`GameplayStatics.PlaySound2D` "/Game/Team9Content/Soude/Porte-Metal.Porte-Metal" 1.0 1.0 0.0 null null)
  (bind (_direction _openthedoor) (`Timeline|openDoor` :!via `PlayFromStart` :!label _label)
    (:`Update`
      (`SceneComponent.K2_SetRelativeRotation` (`self.DoorMesh`) (`KismetMathLibrary.MakeRotator` 0.0 0.0 (`KismetMathLibrary.Lerp` 0.0 90.0 _openthedoor)) false false)
      (`KismetSystemLibrary.Delay` 5.0)
      (`GameplayStatics.PlaySound2D` "/Game/Team9Content/Soude/Porte-Metal.Porte-Metal" 1.0 1.0 0.0 null null)
      (if (`self.Opened`)
        (`self.CE_CloseDoor`)))))

(event `CE_CloseDoor`
  (set `self.Opened` false)
  (goto _label :!via `ReverseFromEnd`))

(event `/Game/Team9Content/BP/Maxime/BPI_Interactable.Interactable`
  (if (not (`self.Opened`))
    (`self.open door`)))

(fn `UserConstructionScript`)