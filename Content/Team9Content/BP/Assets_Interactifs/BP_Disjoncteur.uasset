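; Interactive circuit breaker (disjoncteur) that sets the intensity of every RectLight in the level when used.
; On BeginPlay it gathers all RectLight actors and copies each intensity into one shared variable, so only the last light's value remains.
; The Interactable event applies that stored value to all gathered lights; nothing here dims or switches them off.
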(event `self.ReceiveBeginPlay`
  (bind _outactors (`GameplayStatics.GetAllActorsOfClass` "/Script/Engine.RectLight"))
  (bind _output_get (set `self.Lights` _outactors))
  (for _array_element _output_get
    (set `self.Intensity` (`LightComponentBase.Intensity` (`Light.LightComponent` _array_element)))))

(event `/Game/Team9Content/BP/Maxime/BPI_Interactable.Interactable`
  (for _array_element (`self.Lights`)
    (`LightComponent.SetIntensity` (`Light.LightComponent` _array_element) (`self.Intensity`))))

(fn `UserConstructionScript`)