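; First-person player character with Enhanced Input movement and look, camera-shake head bob and hold-to-interact.
; Each Tick starts a Walk or Idle camera shake based on velocity and CanJump.
; Interactable collision overlaps show a hold prompt; holding swaps it for a timeline-driven progress widget, and completion sends InteractableMessage to the overlapped actor.
; CE_Mort forwards death to the HUD, and BeginPlay caches BP_FireTest actors, unused here.
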(event `self.ReceiveBeginPlay`
  (bind _outactors (`GameplayStatics.GetAllActorsOfClass` "/Game/Team9Content/GUILLAUME/BP/BP_FireTest.BP_FireTest_C"))
  (set `self.firetest` _outactors))

(event `EnhancedInput|/Game/Team9Content/Input/IA_Move`
  (params (ActionValue :type "Vector2D Structure") (ElapsedSeconds :type "Float (double-precision)") (TriggeredSeconds :type "Float (double-precision)") (InputAction :type "InputAction Object Reference" :default "/Game/Team9Content/Input/IA_Move.IA_Move"))
  (:`Triggered`
    (`self.AddMovementInput` (`self.GetActorRightVector`) ActionValue_X)
    (`self.AddMovementInput` (`self.GetActorForwardVector`) ActionValue_Y)))

(event `EnhancedInput|/Game/Team9Content/Input/IA_Look`
  (params (ActionValue :type "Vector2D Structure") (ElapsedSeconds :type "Float (double-precision)") (TriggeredSeconds :type "Float (double-precision)") (InputAction :type "InputAction Object Reference" :default "/Game/Team9Content/Input/IA_Look.IA_Look"))
  (:`Triggered`
    (`self.AddControllerYawInput` ActionValue_X)
    (`self.AddControllerPitchInput` ActionValue_Y)))

(event `self.ReceiveControllerChanged`
  (params (OldController :type "Controller Object Reference") (NewController :type "Controller Object Reference"))
  (bind _asplayer_controller (cast `PlayerController` NewController))
  (`EnhancedInputSubsystemInterface.AddMappingContext` (pcsubsystem `EnhancedInputLocalPlayerSubsystem` _asplayer_controller) "/Game/Team9Content/Input/IMC_FPThidiane.IMC_FPThidiane" 0 (struct)))

(event `HeadBob`
  (bind _returnvalue (`GameplayStatics.GetPlayerController` 0))
  (bind _returnvalue_2 (`KismetMathLibrary.VSize` (`self.GetVelocity`)))
  (if (and (> _returnvalue_2 0.0) (`self.CanJump`))
    (if (< _returnvalue_2 300.0)
      _
      (else
        _))
    (`PlayerController.ClientStartCameraShake` :`self` _returnvalue :`Shake` "/Game/Team9Content/BP/Thidiane/walk.walk_C")
    (else
      (`PlayerController.ClientStartCameraShake` :`self` _returnvalue :`Shake` "/Game/Team9Content/BP/Thidiane/Idle.Idle_C"))))

(event `self.ReceiveTick`
  (params (DeltaSeconds :type "Float (single-precision)"))
  (`self.HeadBob`))

(event `CEStopTimeline`
  (bind (_direction _newtrack_0) (`Timeline|Timeline` :!via `Stop` :!label _label)
    (:`Update`
      (bind _interactingui (`self.InteractingUI`)
        (:`then`
          (set `/Game/Team9Content/BP/Maxime/WBP_Hold.PercentBar` _newtrack_0 _interactingui))
        (:`else`
          (`self.CEStopTimeline`))))))

(event `EnhancedInput|/Game/Team9Content/Input/IA_Interact`
  (params (ActionValue :type Boolean) (ElapsedSeconds :type "Float (double-precision)") (TriggeredSeconds :type "Float (double-precision)") (InputAction :type "InputAction Object Reference" :default "/Game/Team9Content/Input/IA_Interact.IA_Interact"))
  (:`Started`
    (`self.CanHoldUI`
      (:`then`
        (bind _returnvalue (`|CreateWidget` "/Game/Team9Content/BP/Maxime/WBP_Hold.WBP_Hold_C"))
        (bind _output_get (set `self.InteractingUI` _returnvalue))
        (`UserWidget.AddToViewport` _output_get 0)
        (`Widget.RemoveFromParent` (`self.CanHoldUI`))
        (set `self.CanHoldUI` null)
        (goto _label :!via `PlayFromStart`))
      (:`else`)))
  (:`Canceled`
    (bind _interactingui (`self.InteractingUI`)
      (:`then`
        (`Widget.RemoveFromParent` _interactingui)
        (set `self.InteractingUI` null)
        (bind _returnvalue_2 (`|CreateWidget` "/Game/Team9Content/BP/Maxime/WBP_CanHold.WBP_CanHold_C"))
        (bind _output_get_2 (set `self.CanHoldUI` _returnvalue_2))
        (`UserWidget.AddToViewport` _output_get_2 0))
      (:`else`)))
  (:`Completed`
    (bind _interactingui_2 (`self.InteractingUI`)
      (:`then`
        (`Widget.RemoveFromParent` _interactingui_2)
        (set `self.InteractingUI` null)
        (message `/Game/Team9Content/BP/Maxime/BPI_Interactable.Interactable` (stale `self.Interactable Collision.OnComponentBeginOverlap` OtherActor)))
      (:`else`))))

(event `CE_Mort`
  (message `/Game/Team9Content/GUILLAUME/BPI_HUD.Mort` (`PlayerController.GetHUD` (`GameplayStatics.GetPlayerController` 0))))

(event `self.Interactable Collision.OnComponentBeginOverlap`
  (params (OverlappedComponent :type "PrimitiveComponent Object Reference") (OtherActor :type "Actor Object Reference") (OtherComp :type "PrimitiveComponent Object Reference") (OtherBodyIndex :type Integer) (bFromSweep :type Boolean) (SweepResult :type "HitResult Structure (by ref)"))
  (bind _returnvalue (`|CreateWidget` "/Game/Team9Content/BP/Maxime/WBP_CanHold.WBP_CanHold_C"))
  (bind _output_get (set `self.CanHoldUI` _returnvalue))
  (`UserWidget.AddToViewport` _output_get 0))

(event `self.Interactable Collision.OnComponentEndOverlap`
  (params (OverlappedComponent :type "PrimitiveComponent Object Reference") (OtherActor :type "Actor Object Reference") (OtherComp :type "PrimitiveComponent Object Reference") (OtherBodyIndex :type Integer))
  (bind _canholdui (`self.CanHoldUI`)
    (:`then`
      (`Widget.RemoveFromParent` _canholdui)
      (set `self.CanHoldUI` null))
    (:`else`
      (bind _interactingui (`self.InteractingUI`)
        (:`then`
          (`Widget.RemoveFromParent` _interactingui)
          (set `self.InteractingUI` null))
        (:`else`)))))

(fn `UserConstructionScript`)