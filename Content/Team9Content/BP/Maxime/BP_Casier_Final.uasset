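; Interactable locker that randomly becomes trapped and spawns AI when the player fails to handle it correctly.
; A looping 30-second timer re-rolls the trap and notifies listeners by index, first spawning a BP_AI if the previous trap is still active.
; Interacting clears an active trap, while interacting with an untrapped locker spawns one after a short delay.
; Spawned AI appear at the BP_SpawnActor location and receive CEChangeVictime.
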(event `self.ReceiveBeginPlay`
  (`KismetSystemLibrary.Delay` 0.5)
  (`self.TrapCasier`)
  (bind _returnvalue (`KismetSystemLibrary.K2_SetTimerDelegate` (delegate `TrapCasier`) 30.0 true))
  (set `self.TimerHandler` _returnvalue)
  (bind _returnvalue_2 (`GameplayStatics.GetActorOfClass` "/Game/Team9Content/GUILLAUME/BP/BP_SpawnActor.BP_SpawnActor_C"))
  (set `self.Spawn` _returnvalue_2))

(event `TrapCasier`
  (bind _index (`self.index`))
  (`GameplayStatics.PlaySound2D` "/Game/Team9Content/Soude/Casier-Reset.Casier-Reset" 0.05 1.0 0.0 null null)
  (if (`self.istrapped`)
    (bind _returnvalue (`|SpawnActorFromClass` "/Game/Team9Content/GUILLAUME/BP/BP_AI.BP_AI_C" (`SceneComponent.K2_GetComponentToWorld` (`/Game/Team9Content/GUILLAUME/BP/BP_SpawnActor.DefaultSceneRoot` (`self.Spawn`))) "Undefined" "MultiplyWithRoot" null null))
    (`Pawn.SpawnDefaultController` _returnvalue)
    (`/Game/Team9Content/GUILLAUME/BP/BP_AI.CE_ChangeVictime` _returnvalue)
    (`GameplayStatics.PlaySound2D` "/Game/Team9Content/Soude/Cadavre-Tombe-Casier.Cadavre-Tombe-Casier" 1.0 1.0 0.0 null null))
  (if (< (`KismetMathLibrary.RandomIntegerInRange` 1 10) 5)
    (set `self.istrapped` true)
    (`self.ED_Trapped` _index)
    (else
      (set `self.istrapped` false)
      (`self.ED_Untrapped` _index))))

(event `/Game/Team9Content/BP/Maxime/BPI_Interactable.Interactable`
  (if (`self.istrapped`)
    (`KismetSystemLibrary.PrintString` "yipiiii")
    (`self.ED_Untrapped` (`self.index`))
    (set `self.istrapped` false)
    (`GameplayStatics.PlaySound2D` "/Game/Team9Content/Soude/Casier-Kick.Casier-Kick" 1.25 1.0 0.0 null null)
    (else
      (`GameplayStatics.PlaySound2D` "/Game/Team9Content/Soude/Cadavre-Apparition.Cadavre-Apparition" 1.0 1.0 0.0 null null)
      (`KismetSystemLibrary.PrintString` "ah ba non")
      (`KismetSystemLibrary.Delay` 3.0)
      (bind _returnvalue (`|SpawnActorFromClass` "/Game/Team9Content/GUILLAUME/BP/BP_AI.BP_AI_C" (`SceneComponent.K2_GetComponentToWorld` (`/Game/Team9Content/GUILLAUME/BP/BP_SpawnActor.DefaultSceneRoot` (`self.Spawn`))) "Undefined" "MultiplyWithRoot" null null))
      (`Pawn.SpawnDefaultController` _returnvalue)
      (`/Game/Team9Content/GUILLAUME/BP/BP_AI.CE_ChangeVictime` _returnvalue))))

(fn `UserConstructionScript`
  (`parent.UserConstructionScript`))