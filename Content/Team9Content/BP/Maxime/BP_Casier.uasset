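; BP_Casier is a locker that randomly becomes trapped or untrapped during play and responds to interaction.
; Shortly after BeginPlay it rolls its state, then a looping timer rerolls it periodically, broadcasting trapped or untrapped dispatchers with its Index.
; Interacting while trapped broadcasts untrapped but leaves the Istrapped flag set until a roll clears it; both interaction branches print debug strings.
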(event `self.ReceiveBeginPlay`
  (`KismetSystemLibrary.Delay` 0.5)
  (`self.TrapCasier`)
  (bind _returnvalue (`KismetSystemLibrary.K2_SetTimerDelegate` (delegate `TrapCasier`) 20.0 true false 20.0))
  (set `self.TimerHandler` _returnvalue))

(event `TrapCasier`
  (bind _index (`self.index`))
  (if (< (`KismetMathLibrary.RandomIntegerInRange` 0 10) 5)
    (set `self.istrapped` true)
    (`self.ED_Trapped` _index)
    (else
      (set `self.istrapped` false)
      (`self.ED_Untrapped` _index))))

(event `/Game/Team9Content/BP/Maxime/BPI_Interactable.Interactable`
  (if (`self.istrapped`)
    (`KismetSystemLibrary.PrintString` "yipiiii")
    (`self.ED_Untrapped` (`self.index`))
    (else
      (`KismetSystemLibrary.PrintString` "ah ba non"))))

(fn `UserConstructionScript`
  (`parent.UserConstructionScript`))