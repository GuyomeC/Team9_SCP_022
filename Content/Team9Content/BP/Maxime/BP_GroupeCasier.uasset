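; BP_GroupeCasier is a locker group Blueprint that plays random ambient creaking sounds in the game.
; On BeginPlay it starts the ambient noise event and stores every BP_Casier_Final actor in Casier, which this file does not use further.
; The self-calling event waits, then randomly plays one of two creak sounds in 2D or waits again for a second roll before repeating.
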(event `self.ReceiveBeginPlay`
  (`self.CE_BruitAmbiant`)
  (bind _outactors (`GameplayStatics.GetAllActorsOfClass` "/Game/Team9Content/BP/Maxime/BP_Casier_Final.BP_Casier_Final_C"))
  (set `self.Casier` _outactors))

(event `CE_BruitAmbiant`
  (bind _returnvalue (< (`KismetMathLibrary.RandomIntegerInRange` 1 10) 5))
  (`KismetSystemLibrary.Delay` 4.0)
  (if _returnvalue
    (if _returnvalue
      (`GameplayStatics.PlaySound2D` "/Game/Team9Content/Soude/Bruit-Craquement-1.Bruit-Craquement-1" 1.0 1.0 0.0 null null)
      (else
        (`GameplayStatics.PlaySound2D` "/Game/Team9Content/Soude/Bruits-Craquement-2.Bruits-Craquement-2" 1.0 1.0 0.0 null null)))
    (`self.CE_BruitAmbiant`)
    (else
      (`KismetSystemLibrary.Delay` 2.0)
      (if _returnvalue
        (if _returnvalue
          (`GameplayStatics.PlaySound2D` "/Game/Team9Content/Soude/Bruit-Craquement-1.Bruit-Craquement-1" 1.0 1.0 0.0 null null)
          (else
            (`GameplayStatics.PlaySound2D` "/Game/Team9Content/Soude/Bruits-Craquement-2.Bruits-Craquement-2" 1.0 1.0 0.0 null null)))
        (`self.CE_BruitAmbiant`)
        (else
          (`self.CE_BruitAmbiant`))))))

(fn `UserConstructionScript`)