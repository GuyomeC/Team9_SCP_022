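; First-person player pawn with Enhanced Input movement, mouse-look style camera control and camera-shake head bob.
; On controller change it adds the IMC_FPThidiane mapping context, and the move and look actions drive movement input and controller yaw and pitch.
; HeadBob runs every tick, starting a Walk shake while moving or an Idle shake when still.
; Its 300-speed check has empty branches, so all movement uses Walk.
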(event `self.ReceiveTick`
  (params (DeltaSeconds :type "Float (single-precision)"))
  (`self.HeadBob`))

(event `EnhancedInput|/Game/Team9Content/Input/IA_Move`
  (params (ActionValue :type "Vector2D Structure") (ElapsedSeconds :type "Float (double-precision)") (TriggeredSeconds :type "Float (double-precision)") (InputAction :type "InputAction Object Reference" :default "/Game/Team9Content/Input/IA_Move.IA_Move"))
  (:`Triggered`
    (`self.AddMovementInput` (`self.GetActorRightVector`) ActionValue_X)
    (`self.AddMovementInput` (`self.GetActorForwardVector`) ActionValue_Y)))

(event `EnhancedInput|/Game/Team9Content/Input/IA_Look`
  (params (ActionValue :type "Vector2D Structure") (ElapsedSeconds :type "Float (double-precision)") (TriggeredSeconds :type "Float (double-precision)") (InputAction :type "InputAction Object Reference" :default "/Game/Team9Content/Input/IA_Look.IA_Look"))
  (:`Triggered`
    (`self.AddControllerYawInput` ActionValue_X)
    (`self.AddControllerPitchInput` ActionValue_Y)))

(event `self.ReceiveControllerChanged`
  (params (OldController :type "Controller Object Reference") (NewController :type "Controller Object Reference"))
  (bind _asplayer_controller (cast `PlayerController` NewController))
  (`EnhancedInputSubsystemInterface.AddMappingContext` (pcsubsystem `EnhancedInputLocalPlayerSubsystem` _asplayer_controller) "/Game/Team9Content/Input/IMC_FPThidiane.IMC_FPThidiane" 0 (struct)))

(event `HeadBob`
  (bind _returnvalue (`GameplayStatics.GetPlayerController` 0))
  (bind _returnvalue_2 (`KismetMathLibrary.VSize` (`self.GetVelocity`)))
  (if (> _returnvalue_2 0.0)
    (if (< _returnvalue_2 300.0)
      _
      (else
        _))
    (`PlayerController.ClientStartCameraShake` :`self` _returnvalue :`Shake` "/Game/Team9Content/BP/Thidiane/walk.walk_C")
    (else
      (`PlayerController.ClientStartCameraShake` :`self` _returnvalue :`Shake` "/Game/Team9Content/BP/Thidiane/Idle.Idle_C"))))

(fn `UserConstructionScript`)