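; BP_FireTest is a test fire ability that blacks out the level's RectLights while on a cooldown.
; BeginPlay caches all RectLight actors; Activate, if allowed, raises IsActive for half a second, then zeroes each light's intensity.
; Desactivate, called inside that loop, blocks reuse for ten seconds, then applies one shared saved intensity to every light rather than per-light values.
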(event `self.ReceiveBeginPlay`
  (set `self.IsActive` false)
  (set `self.CanUseFire` true)
  (bind _outactors (`GameplayStatics.GetAllActorsOfClass` "/Script/Engine.RectLight"))
  (set `self.Lights` _outactors))

(event `/Game/Team9Content/GUILLAUME/BPI_Fire.Activate`
  (if (`self.CanUseFire`)
    (set `self.IsActive` true)
    (`KismetSystemLibrary.Delay` 0.5)
    (set `self.IsActive` false)
    (for _array_element (`self.Lights`)
      (bind _lightcomponent (`Light.LightComponent` _array_element))
      (set `self.Intensity` (`LightComponentBase.Intensity` _lightcomponent))
      (`LightComponent.SetIntensity` _lightcomponent 0.0)
      (`self.Desactivate`))))

(event `/Game/Team9Content/GUILLAUME/BPI_Fire.Desactivate`
  (set `self.CanUseFire` false)
  (`KismetSystemLibrary.Delay` 10.0)
  (set `self.CanUseFire` true)
  (for _array_element (`self.Lights`)
    (`LightComponent.SetIntensity` (`Light.LightComponent` _array_element) (`self.Intensity`))))

(fn `UserConstructionScript`)