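; Child character Blueprint that extends the Thidiane character with debug hotkeys for fire and corpse-zone test gameplay.
; On BeginPlay it caches the first BP_FireTest and BP_ZoneCadavreTest actors in the level.
; T calls ActivateMessage on the fire actor.
; B, when IsInZone is set, prints a placeholder aiming-game message and resets camera world rotation by briefly disabling pawn control rotation.
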(event `self.ReceiveBeginPlay`
  (`parent.ReceiveBeginPlay`)
  (bind _returnvalue (`GameplayStatics.GetActorOfClass` "/Game/Team9Content/GUILLAUME/BP/BP_FireTest.BP_FireTest_C"))
  (set `self.firetest` _returnvalue)
  (bind _returnvalue_2 (`GameplayStatics.GetActorOfClass` "/Game/Team9Content/GUILLAUME/BP/BP_ZoneCadavreTest.BP_ZoneCadavreTest_C"))
  (set `self.zonecadavre` _returnvalue_2))

(event `self.ReceiveActorBeginOverlap`
  (params (OtherActor :type "Actor Object Reference"))
  (`parent.ReceiveActorBeginOverlap` OtherActor))

(event `self.ReceiveTick`
  (params (DeltaSeconds :type "Float (single-precision)"))
  (`parent.ReceiveTick` DeltaSeconds))

(event `Key|T`
  (params (Key :type "Key Structure"))
  (:`Pressed`
    (message `/Game/Team9Content/GUILLAUME/BPI_Fire.Activate` (`self.firetest`))))

(event `Key|B`
  (params (Key :type "Key Structure"))
  (bind _camera (`self.Camera`))
  (:`Pressed`
    (if (`self.IsInZone`)
      (`KismetSystemLibrary.PrintString` "jeu de visé")
      (set `CameraComponent.bUsePawnControlRotation` false _camera)
      (`SceneComponent.K2_SetWorldRotation` :`self` _camera)
      (set `CameraComponent.bUsePawnControlRotation` true _camera)
      (else
        (`KismetSystemLibrary.PrintString` "non")))))

(fn `UserConstructionScript`
  (`parent.UserConstructionScript`))