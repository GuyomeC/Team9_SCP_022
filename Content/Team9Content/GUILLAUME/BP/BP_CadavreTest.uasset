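; BP_CadavreTest is a test corpse actor that slides along X and can be destroyed by fire.
; On BeginPlay it moves its Cube component forward over a fixed time, then prints an arrival message.
; Box overlaps with a BP_FireTest store that actor and set an in-zone flag, which any end overlap clears.
; Tick destroys the corpse while it is flagged in the zone and the stored fire is active.
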(event `self.ReceiveBeginPlay`
  (bind _cube (`self.Cube`))
  (bind (_relativelocation_x _relativelocation_y _relativelocation_z) (`KismetMathLibrary.BreakVector` (`SceneComponent.RelativeLocation` _cube)))
  (set `self.IsInFireZone` false)
  (`KismetSystemLibrary.MoveComponentTo` _cube (`KismetMathLibrary.MakeVector` (+ _relativelocation_x 2000.0) _relativelocation_y _relativelocation_z) (struct) false false 10.0)
  (`KismetSystemLibrary.PrintString` "Arriver"))

(event `self.Box.OnComponentBeginOverlap`
  (params (OverlappedComponent :type "PrimitiveComponent Object Reference") (OtherActor :type "Actor Object Reference") (OtherComp :type "PrimitiveComponent Object Reference") (OtherBodyIndex :type Integer) (bFromSweep :type Boolean) (SweepResult :type "HitResult Structure (by ref)"))
  (bind _asbp_fire_test (cast `/Game/Team9Content/GUILLAUME/BP/BP_FireTest` OtherActor))
  (set `self.As BP Fire Test` _asbp_fire_test)
  (set `self.IsInFireZone` true))

(event `self.Box.OnComponentEndOverlap`
  (params (OverlappedComponent :type "PrimitiveComponent Object Reference") (OtherActor :type "Actor Object Reference") (OtherComp :type "PrimitiveComponent Object Reference") (OtherBodyIndex :type Integer))
  (set `self.IsInFireZone` false))

(event `self.ReceiveTick`
  (params (DeltaSeconds :type "Float (single-precision)"))
  (if (`self.IsInFireZone`)
    (if (`/Game/Team9Content/GUILLAUME/BP/BP_FireTest.IsActive` (`self.As BP Fire Test`))
      (`self.K2_DestroyActor`))))

(fn `UserConstructionScript`)