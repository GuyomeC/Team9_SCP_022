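; BP_ZoneCadavreTest is a test zone actor that tracks whether the BP_CharacterThidiane_Child character is inside its Box.
; Begin overlap casts and caches the character, sets its IsInZone flag and prints a debug string.
; End overlap prints and clears the flag on the cached reference without checking which actor left.
; BeginPlay stores a GetActorOfClass result in Location, which is otherwise unused here.
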(event `self.ReceiveBeginPlay`
  (bind _returnvalue (`GameplayStatics.GetActorOfClass` "/Game/Team9Content/GUILLAUME/BP/Location.Location_C"))
  (set `self.location` _returnvalue))

(event `self.Box.OnComponentBeginOverlap`
  (params (OverlappedComponent :type "PrimitiveComponent Object Reference") (OtherActor :type "Actor Object Reference") (OtherComp :type "PrimitiveComponent Object Reference") (OtherBodyIndex :type Integer) (bFromSweep :type Boolean) (SweepResult :type "HitResult Structure (by ref)"))
  (bind _asbp_character_thidiane_child (cast `/Game/Team9Content/GUILLAUME/BP/BP_CharacterThidiane_Child` OtherActor))
  (bind _output_get (set `self.As BP Character Thidiane Child` _asbp_character_thidiane_child))
  (set `/Game/Team9Content/GUILLAUME/BP/BP_CharacterThidiane_Child.IsInZone` true _output_get)
  (`KismetSystemLibrary.PrintString` "rentrer"))

(event `self.Box.OnComponentEndOverlap`
  (params (OverlappedComponent :type "PrimitiveComponent Object Reference") (OtherActor :type "Actor Object Reference") (OtherComp :type "PrimitiveComponent Object Reference") (OtherBodyIndex :type Integer))
  (`KismetSystemLibrary.PrintString` "sorti")
  (set `/Game/Team9Content/GUILLAUME/BP/BP_CharacterThidiane_Child.IsInZone` false (`self.As BP Character Thidiane Child`)))

(fn `UserConstructionScript`)